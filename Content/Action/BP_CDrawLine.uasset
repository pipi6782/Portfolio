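; BP_CDrawLine is a line-drawing Blueprint that builds a spline with meshes from locations passed to its Draw event.
; Draw calls the parent, appends the world location as a spline point, then runs AddSplineComponent.
; That function adds an X-forward spline mesh spanning the first to last point, rather than just the newest segment, and prints a debug string.
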(event EventTick
  (params (DeltaSeconds :type Float%20%28single-precision%29))
  (|CallParentFunction DeltaSeconds))

(event EventBeginPlay
  (|CallParentFunction))

(event EventDraw
  (params (InLocation :type Vector%20%28by%20ref%29 :default "0, 0, 0"))
  (|CallParentFunction InLocation)
  (Spline|AddSplinePoint (Variables|Default|GetSpline) InLocation "World" true)
  (|AddSplineComponent))

(fn ConstructionScript)